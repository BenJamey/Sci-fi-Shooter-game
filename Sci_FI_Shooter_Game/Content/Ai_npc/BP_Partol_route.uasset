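; BP_Partol_route is a patrol route Blueprint for AI NPCs, defined by a spline.
; It tracks a current point index and returns that spline point's world position on request.
; An increment event advances the index by a direction value and prints it for debugging, with no bounds check or reversal wired in.
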(event `IncermentPatrolRoute`
  (set `self.PatrolIndex` (+ (`self.PatrolIndex`) (`self.Direction`)))
  (`KismetSystemLibrary.PrintString` (`KismetStringLibrary.Concat_StrStr` "Patrol Index =" (`KismetStringLibrary.Conv_IntToString` (`self.PatrolIndex`)))))

(fn `GetSplinePonitAsWorldPos`
  (returns (Location :type "Vector Structure"))
  (return (`SplineComponent.GetLocationAtSplinePoint` (`self.PatrolRoute`) (`self.PatrolIndex`) "World")))

(fn `UserConstructionScript`)
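; BP_Ai is an NPC character that can throw a punch, expose a patrol route and change movement speed.
; The Attack event plays a punch montage on the mesh and fires the OnAttackEnd dispatcher whether it completes or is interrupted.
; GetPatrolRoute returns the stored route, while SetMovementSpeed maps an idle, walking or sprinting state to the character's max walk speed and returns it.
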(event `self.ReceiveBeginPlay`)

(event `Attack`
  (`|PlayMontage` (`self.Mesh`) "/Game/Characters/MixamoCharacters/Alien_Soldier/Ani_montage_punch.Ani_montage_punch" 1.0 0.0 "None" false
    (:`OnCompleted`
      _)
    (:`OnInterrupted`
      _))
  (`self.OnAttackEnd`))

(fn `GetPatrolRoute`
  (returns (PatrolRoute :type "/Game/Ai_npc/BP_Partol_route Object Reference"))
  (return (`self.PatrolRoute`)))

(fn `SetMovementSpeed`
  (params (Speed :type "/Game/Ai_npc/Enums/E_MovementSpeed Enum" :default "NewEnumerator0"))
  (returns (SpeedValue :type "Float (double-precision)"))
  (bind _output_get (set `CharacterMovementComponent.MaxWalkSpeed` (select `/Game/Ai_npc/Enums/E_MovementSpeed` Speed :`NewEnumerator1` 150.0 :`NewEnumerator2` 450.0 :!type "Float (single-precision)") (`self.CharacterMovement`)))
  (return _output_get))

(fn `UserConstructionScript`)